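; Player actor that moves in discrete steps on the XZ plane and collects energy cells by attaching them to itself.
; Directional inputs store previous location and sweep to a floored position, which CancelMove can revert.
; Box overlaps attach cells offset along the move direction, or destroy them if CanAttractCell is unset, as when spawned on the player.
; Each tick, the camera shifts toward the mouse relative to screen center.
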(event `InputAction|MoveRight`
  (params (Key :type "Key Structure"))
  (:`Pressed`
    (bind _output_get (set `self.MoveDirection` (`KismetMathLibrary.MakeVector` 1.0)))
    (`self.MoveToUnit` _output_get)))

(event `InputAction|MoveTop`
  (params (Key :type "Key Structure"))
  (:`Pressed`
    (bind _output_get (set `self.MoveDirection` (`KismetMathLibrary.MakeVector` 0.0 0.0 1.0)))
    (`self.MoveToUnit` _output_get)))

(event `InputAction|MoveBottom`
  (params (Key :type "Key Structure"))
  (:`Pressed`
    (bind _output_get (set `self.MoveDirection` (`KismetMathLibrary.MakeVector` 0.0 0.0 -1.0)))
    (`self.MoveToUnit` _output_get)))

(event `InputAction|MoveLeft`
  (params (Key :type "Key Structure"))
  (:`Pressed`
    (bind _output_get (set `self.MoveDirection` (`KismetMathLibrary.MakeVector` -1.0)))
    (`self.MoveToUnit` _output_get)))

(event `self.ReceiveTick`
  (params (DeltaSeconds :type "Float (single-precision)"))
  (bind _returnvalue (`self.GetCamOffset`))
  (`SceneComponent.K2_SetRelativeLocation` (`self.Camera`) _returnvalue true false))

(event `self.Box.OnComponentBeginOverlap`
  (params (OverlappedComponent :type "PrimitiveComponent Object Reference") (OtherActor :type "Actor Object Reference") (OtherComp :type "PrimitiveComponent Object Reference") (OtherBodyIndex :type Integer) (bFromSweep :type Boolean) (SweepResult :type "HitResult Structure (by ref)"))
  ;[1 1 1] Energy Cell Attraction
  (bind _asbp_energy_cell (cast `/Game/Blueprints/Cells/BP_EnergyCell` OtherActor))
  (if (`self.CanAttractCell`)
    (`self.AttractEnergyCell` _asbp_energy_cell)
    (else
      (`self.K2_DestroyActor` _asbp_energy_cell) ; Destroy cells that spawn on player
    )))

(fn `AttractEnergyCell`
  (params (EnergyCell :type "/Game/Blueprints/Cells/BP_EnergyCell Object Reference"))
  (locals (CellToAttract :type "/Game/Blueprints/Cells/BP_EnergyCell Object Reference"))
  (bind _output_get (set `local.CellToAttract` EnergyCell))
  (`/Game/Blueprints/Cells/BP_EnergyCell.AttachToPlayer` _output_get self)
  (`PrimitiveComponent.SetCollisionResponseToChannel` (`self.GetComponentByClass` (`local.CellToAttract`) "/Script/Engine.BoxComponent") "ECC_Pawn" "ECR_Ignore")
  (`self.K2_SetActorLocation` (`local.CellToAttract`) (+ (`self.K2_GetActorLocation` (`local.CellToAttract`)) (`self.MoveDirection`)) false true)
  (`self.K2_AttachToComponent` (`local.CellToAttract`) (`self.RootComponent`) "None" "KeepWorld" "KeepRelative" "KeepRelative" true))

(fn `CancelMove`
  (`self.K2_SetActorLocation` (`self.PreviousLocation`) false true))

(fn `GetCamOffset`
  (returns (ReturnValue :type "Vector Structure"))
  (locals (Thresold :type "Vector2D Structure") (Mouse :type "Vector2D Structure"))
  (bind (_locationx _locationy) (`PlayerController.GetMousePosition` (`GameplayStatics.GetPlayerController` 0)))
  (bind (_x _y) (`KismetMathLibrary.BreakVector2D` (`local.Mouse`)))
  (bind (_x_2 _y_2) (`KismetMathLibrary.BreakVector2D` (`local.Mouse`)))
  (bind _returnvalue (* (`WidgetLayoutLibrary.GetViewportSize`) (0.5 0.5)))
  (bind (_x_3 _y_3) (`KismetMathLibrary.BreakVector2D` _returnvalue))
  (bind (_x_4 _y_4) (`KismetMathLibrary.BreakVector2D` (* (/ (`KismetMathLibrary.MakeVector2D` (- _x _x_3) (- _y_3 _y)) _returnvalue) (`self.MaxCamDistance`))))
  ;[1 1 1] Refresh mouse position
  (set `local.Mouse` (`KismetMathLibrary.MakeVector2D` _locationx _locationy))
  (if (or (> _x_2 0.0) (> _y_2 0.0))
    ;[1 1 1] Refresh mouse position if on screen
    (set `self.CamOffset` (`KismetMathLibrary.MakeVector` _x_4 0.0 _y_4)))
  (return (`self.CamOffset`)))

(fn `MoveToUnit`
  (params (Direction :type "Vector Structure"))
  (set `self.CanAttractCell` true)
  (set `self.PreviousLocation` (`self.K2_GetActorLocation`))
  (`self.K2_SetActorLocation` (`KismetMathLibrary.MakeVector` (`KismetMathLibrary.Conv_IntToDouble` (`KismetMathLibrary.FFloor` (.x (+ (`self.K2_GetActorLocation`) (* Direction (`self.MoveScale`)))))) (`KismetMathLibrary.Conv_IntToDouble` (`KismetMathLibrary.FFloor` (.y (+ (`self.K2_GetActorLocation`) (* Direction (`self.MoveScale`)))))) (`KismetMathLibrary.Conv_IntToDouble` (`KismetMathLibrary.FFloor` (.z (+ (`self.K2_GetActorLocation`) (* Direction (`self.MoveScale`))))))) true))

(fn `UserConstructionScript`
  (`self.K2_SetActorLocation` (0.0 0.0 0.0)))