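; Player Paper2D character that moves in discrete steps on the X-Z plane, one step per press of the four directional input actions.
; Each action passes a unit direction to MoveToUnit, which scales it by MoveScale and adds it to the actor location.
; The result is floored to whole units and applied with a swept SetActorLocation, setting position directly without using movement input.
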(fn `MoveToUnit`
  (params (A :type "Vector Structure"))
  (`self.K2_SetActorLocation` (`KismetMathLibrary.MakeVector` (`KismetMathLibrary.Conv_IntToDouble` (`KismetMathLibrary.FFloor` (.x (+ (`self.K2_GetActorLocation`) (* A (`self.MoveScale`)))))) (`KismetMathLibrary.Conv_IntToDouble` (`KismetMathLibrary.FFloor` (.y (+ (`self.K2_GetActorLocation`) (* A (`self.MoveScale`)))))) (`KismetMathLibrary.Conv_IntToDouble` (`KismetMathLibrary.FFloor` (.z (+ (`self.K2_GetActorLocation`) (* A (`self.MoveScale`))))))) true))

(fn `UserConstructionScript`)