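; BP_EnergyCellsSpawner scatters BP_EnergyCell actors across a grid in the XZ plane when play begins.
; Nested column and row loops offset from a grid origin derived from GridCenterPos, the grid counts and cell size.
; Each spawn lands at a random integer position within its cell at Y zero, giving a jittered-grid distribution.
; Once spawning finishes, the spawner destroys its DefaultSceneRoot component.
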(event `self.ReceiveBeginPlay`
  (bind _returnvalue (* (`self.CurrenRow`) (`self.GridCellSize`)))
  (bind _returnvalue_2 (* (`self.CurrentColumn`) (`self.GridCellSize`)))
  (for _index (range (+ (`self.NbColumns`) 1))
    (set `self.CurrentColumn` _index)
    (for _index_2 (range (+ (`self.NbRows`) 1))
      (set `self.CurrenRow` _index_2)
      (`|SpawnActorFromClass` "/Game/Blueprints/BP_EnergyCell.BP_EnergyCell_C" (`KismetMathLibrary.MakeTransform` (`KismetMathLibrary.MakeVector` (+ (.x (`KismetMathLibrary.MakeVector` (- (.x (`self.GridCenterPos`)) (`KismetMathLibrary.Conv_IntToDouble` (/ (* (`self.NbColumns`) (`self.GridCellSize`)) 2))) (.y (`self.GridCenterPos`)) (- (.z (`self.GridCenterPos`)) (`KismetMathLibrary.Conv_IntToDouble` (/ (* (`self.NbRows`) (`self.GridCellSize`)) 2))))) (`KismetMathLibrary.Conv_IntToDouble` (`KismetMathLibrary.RandomIntegerInRange` _returnvalue_2 (+ _returnvalue_2 (`self.GridCellSize`))))) 0.0 (+ (.z (`KismetMathLibrary.MakeVector` (- (.x (`self.GridCenterPos`)) (`KismetMathLibrary.Conv_IntToDouble` (/ (* (`self.NbColumns`) (`self.GridCellSize`)) 2))) (.y (`self.GridCenterPos`)) (- (.z (`self.GridCenterPos`)) (`KismetMathLibrary.Conv_IntToDouble` (/ (* (`self.NbRows`) (`self.GridCellSize`)) 2))))) (`KismetMathLibrary.Conv_IntToDouble` (`KismetMathLibrary.RandomIntegerInRange` _returnvalue (+ _returnvalue (`self.GridCellSize`))))))) "Undefined" "OverrideRootScale" null null)))
  (`ActorComponent.K2_DestroyComponent` (`self.DefaultSceneRoot`)))

(fn `UserConstructionScript`)