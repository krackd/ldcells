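; Crosshair cursor actor that replaces the mouse pointer with a sprite while offensive mode is active.
; BeginPlay binds to BP_InputsManager's offensive mode events, which toggle the default cursor and sprite visibility.
; Mouse movement deprojects the pointer to world space, truncating X and Z to whole units on the Y=0 plane for snapping.
; Both handlers set IsOffensiveMode true, so position tracking continues after the mode is disabled.
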(event `self.ReceiveBeginPlay`
  ;[1 1 1] Bind to offensive mode events
  (bind _outactors (`GameplayStatics.GetAllActorsOfClass` "/Game/Blueprints/Inputs/BP_InputsManager.BP_InputsManager_C"))
  (bind _output (`|GetArrayItem` _outactors))
  (add `/Game/Blueprints/Inputs/BP_InputsManager.OnOffensiveModeEnabled` _output (delegate `OnOffensiveModeEnabled_Event`))
  (add `/Game/Blueprints/Inputs/BP_InputsManager.OnOffensiveModeDisabled` _output (delegate `OnOffensiveModeDisabled_Event`)))

(event `OnOffensiveModeEnabled_Event`
  (bind _returnvalue (`GameplayStatics.GetPlayerController` 0))
  ;[1 1 1] Store offensive mode state
  (set `self.IsOffensiveMode` true)
  ;[1 1 1] Hide/show crosshair
  (set `PlayerController.CurrentMouseCursor` "None" _returnvalue)
  (`SceneComponent.SetVisibility` (`self.CursorSprite`) true false)
  (`self.UpdateSnappedLocation` _returnvalue))

(event `OnOffensiveModeDisabled_Event`
  ;[1 1 1] Store offensive mode state
  (set `self.IsOffensiveMode` true)
  ;[1 1 1] Hide/show crosshair
  (set `PlayerController.CurrentMouseCursor` "Default" (`GameplayStatics.GetPlayerController` 0))
  (`SceneComponent.SetVisibility` (`self.CursorSprite`) false false))

(event `InputAxisKey|MouseX`
  (params (AxisValue :type "Float (single-precision)"))
  ;[1 1 1] Update crosshair sprite position
  (if (`self.IsOffensiveMode`) :!label _label
    (`self.UpdateSnappedLocation` (`GameplayStatics.GetPlayerController` 0))))

(event `InputAxisKey|MouseY`
  (params (AxisValue :type "Float (single-precision)"))
  ;[1 1 1] Update crosshair sprite position
  (goto _label))

(fn `UpdateSnappedLocation`
  (params (playerController :type "PlayerController Object Reference"))
  (`SceneComponent.K2_SetWorldLocation` (`self.RootComponent`) (`KismetMathLibrary.MakeVector` (`KismetMathLibrary.Conv_IntToDouble` (`KismetMathLibrary.FTrunc` (.x (`PlayerController.DeprojectMousePositionToWorld` playerController)))) 0.0 (`KismetMathLibrary.Conv_IntToDouble` (`KismetMathLibrary.FTrunc` (.z (`PlayerController.DeprojectMousePositionToWorld` playerController))))) false true))

(fn `UserConstructionScript`)