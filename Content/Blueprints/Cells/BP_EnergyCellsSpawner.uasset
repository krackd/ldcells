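; BP_EnergyCellsSpawner scatters BP_EnergyCell actors over a grid centered on itself in the XZ plane at Y=0.
; On BeginPlay it spawns one cell per row and column slot, jittered to a random integer position within that slot.
; Each cell receives the shared resource value and a random type from five, then refreshes its flipbook.
; The spawner then destroys its root component.
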(event `self.ReceiveBeginPlay`
  (bind _returnvalue (* (- (`self.CurrenRow`) 1) (`self.GridCellSize`)))
  (bind _returnvalue_2 (* (- (`self.CurrentColumn`) 1) (`self.GridCellSize`)))
  (for _index (range 1 (+ (`self.NbColumns`) 1))
    (set `self.CurrentColumn` _index)
    (for _index_2 (range 1 (+ (`self.NbRows`) 1))
      (set `self.CurrenRow` _index_2)
      (bind _returnvalue_3 (`|SpawnActorFromClass` "/Game/Blueprints/Cells/BP_EnergyCell.BP_EnergyCell_C" (`KismetMathLibrary.MakeTransform` (`KismetMathLibrary.MakeVector` (+ (.x (`KismetMathLibrary.MakeVector` (- (.x (`self.K2_GetActorLocation`)) (`KismetMathLibrary.Conv_IntToDouble` (/ (* (`self.NbColumns`) (`self.GridCellSize`)) 2))) (.y (`self.K2_GetActorLocation`)) (- (.z (`self.K2_GetActorLocation`)) (`KismetMathLibrary.Conv_IntToDouble` (/ (* (`self.NbRows`) (`self.GridCellSize`)) 2))))) (`KismetMathLibrary.Conv_IntToDouble` (`KismetMathLibrary.RandomIntegerInRange` _returnvalue_2 (+ _returnvalue_2 (`self.GridCellSize`))))) 0.0 (+ (.z (`KismetMathLibrary.MakeVector` (- (.x (`self.K2_GetActorLocation`)) (`KismetMathLibrary.Conv_IntToDouble` (/ (* (`self.NbColumns`) (`self.GridCellSize`)) 2))) (.y (`self.K2_GetActorLocation`)) (- (.z (`self.K2_GetActorLocation`)) (`KismetMathLibrary.Conv_IntToDouble` (/ (* (`self.NbRows`) (`self.GridCellSize`)) 2))))) (`KismetMathLibrary.Conv_IntToDouble` (`KismetMathLibrary.RandomIntegerInRange` _returnvalue (+ _returnvalue (`self.GridCellSize`)))))) (struct) (1.0 1.0 1.0)) "Undefined" "OverrideRootScale" null null))
      (`/Engine/EditorBlueprintResources/StandardMacros.IsValid` _returnvalue_3
        (:`Is Valid`
          (set `/Game/Blueprints/Cells/BP_EnergyCell.ResourceValue` (`self.ResourcesValue`) _returnvalue_3)
          (set `/Game/Blueprints/Cells/BP_EnergyCell.CellType` (`BlueprintMapLibrary.Map_Find` (`|MakeMap` 0 "NewEnumerator0" 1 "NewEnumerator1" 2 "NewEnumerator2" 3 "NewEnumerator3" 4 "NewEnumerator4" :!valuetype "/Game/Blueprints/Cells/ECellType Enum") (`KismetMathLibrary.RandomInteger` 5)) _returnvalue_3)
          (`/Game/Blueprints/Cells/BP_EnergyCell.UpdateResourceFlipbook` _returnvalue_3)))))
  (`ActorComponent.K2_DestroyComponent` (`self.DefaultSceneRoot`)))

(fn `UserConstructionScript`)