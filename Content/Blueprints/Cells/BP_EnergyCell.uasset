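; Paper2D energy cell that players attach, select and fire, carrying a resource value that doubles on merging.
; A state enum drives it through Free, Attracted, Selected to Fire, Firing and Slag.
; Held cells' overlaps attract other cells, optionally auto-merge, or cancel player movement at walls.
; Fired cells sweep forward on Tick until range or impact, then snap to whole-unit coordinates as Slag until a timer frees them.
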(event `self.ReceiveTick`
  (params (DeltaSeconds :type "Float (single-precision)"))
  (switch `/Game/Blueprints/Cells/ECellState` (`self.CellState`)
    (:`NewEnumerator3`
      (bind _returnvalue (`self.IsStillInFireRange`))
      (if _returnvalue
        ;[1 1 1] Do fire
        (`self.K2_AddActorWorldOffset` (* (`self.FireDirection`) (`self.FireForce`)) true)
        (set `self.FireDistance` (+ (`self.FireDistance`) (`self.FireForce`)))
        (else
          (`self.SetSlag`))))))

(event `self.Box.OnComponentBeginOverlap`
  (params (OverlappedComponent :type "PrimitiveComponent Object Reference") (OtherActor :type "Actor Object Reference") (OtherComp :type "PrimitiveComponent Object Reference") (OtherBodyIndex :type Integer) (bFromSweep :type Boolean) (SweepResult :type "HitResult Structure (by ref)"))
  (bind _currentplayer (`self.CurrentPlayer`))
  ;[1 1 1] Collisions
  (switch `/Game/Blueprints/Cells/ECellState` (`self.CellState`)
    (:`NewEnumerator1`
      (`|ExecutionSequence` :!label _label
        (:`then_0`
          (`/Engine/EditorBlueprintResources/StandardMacros.IsValid` (`self.CurrentPlayer`)
            (:`Is Valid`
              (bind _asbp_energy_cell (cast `/Game/Blueprints/Cells/BP_EnergyCell` OtherActor))
              (`/Game/Blueprints/Player/BP_Custom_Player.AttractEnergyCell` (`self.CurrentPlayer`) _asbp_energy_cell)
              ;[1 1 1] Auto-merge
              (if (`/Game/Blueprints/Player/BP_Custom_Player.IsAutoMerge` (`self.CurrentPlayer`))
                (bind _canmerge (`/Game/Blueprints/Player/BP_Custom_Player.CanMerge` (`self.CurrentPlayer`) self _asbp_energy_cell)) ; TODO externalize this
                (if _canmerge
                  (`/Game/Blueprints/Player/BP_Custom_Player.MergeResources` (`self.CurrentPlayer`) self _asbp_energy_cell))))))
        (:`then_1`
          (cast `/Game/Blueprints/Walls/BP_Wall` OtherActor)
          (`/Engine/EditorBlueprintResources/StandardMacros.IsValid` _currentplayer
            (:`Is Valid`
              (`/Game/Blueprints/Player/BP_Custom_Player.CancelMove` _currentplayer))))))
    (:`NewEnumerator2`
      (goto _label))
    (:`NewEnumerator3`
      (if (!= OtherActor (`self.CurrentPlayer`))
        (bind _asbp_energy_cell_2 (cast `/Game/Blueprints/Cells/BP_EnergyCell` OtherActor)
          (:`then`
            (switch `/Game/Blueprints/Cells/ECellState` (`/Game/Blueprints/Cells/BP_EnergyCell.CellState` _asbp_energy_cell_2) ; Do not stop if colliding with cells which are being fired too
              (:`NewEnumerator0`
                _)
              (:`NewEnumerator4`
                _))
            (`|ExecutionSequence`
              (:`then_0`
                _)))
          (:`CastFailed`
            _))
        ;[1 1 1] Stop firing
        (`self.K2_AddActorWorldOffset` (* (`self.FireDirection`) -0.4))
        (`self.SetSlag`)))))

(fn `AttachToPlayer`
  (params (Player :type "/Game/Blueprints/Player/BP_Custom_Player Object Reference"))
  (set `self.CurrentPlayer` Player)
  (set `self.CellState` "NewEnumerator1")
  (`PaperFlipbookComponent.SetFlipbook` (`self.Flipbook`) "/Game/Graphics/Space/Flipbooks/FP_attracted.FP_attracted")
  (`self.PlayRandom` (`|MakeArray` (`self.attract1`) (`self.attract2`))))

(fn `DettachFromPlayer`
  (`SceneComponent.K2_DetachFromComponent` (`self.Box`) "KeepWorld" "KeepWorld" "KeepWorld" false)
  (`PaperFlipbookComponent.SetFlipbook` (`self.Flipbook`) "/Game/Graphics/Space/Flipbooks/FP_empty.FP_empty"))

(fn `FireCell`
  (params (Direction :type "Vector Structure") (Force :type "Float (double-precision)"))
  (set `self.FireDirection` Direction)
  (set `self.FireForce` Force)
  (`self.DettachFromPlayer`)
  (set `self.CellState` "NewEnumerator3")
  (`PaperFlipbookComponent.SetFlipbook` (`self.Flipbook`) "/Game/Graphics/Space/Flipbooks/FP_selected.FP_selected"))

(fn `IsFreeForFire`
  (returns (IsSelected :type Boolean))
  (return (`|EnumInequality` (`self.CellState`) "NewEnumerator2")))

(fn `IsOwnedByPlayer`
  (params (Index :type Integer))
  (returns (IsOwned :type Boolean))
  (locals (Result :type Boolean))
  (`/Engine/EditorBlueprintResources/StandardMacros.IsValid` (`self.CurrentPlayer`)
    (:`Is Valid`
      (if (== (`GameplayStatics.GetPlayerController` Index) (`Pawn.GetController` (`self.CurrentPlayer`)))
        (set `local.Result` true)
        (return (stale _output_get))))
    (:`Is Not Valid`
      (bind _output_get (set `local.Result` false))
      (return _output_get))))

(fn `IsSelectedToFire`
  (returns (IsSelected :type Boolean))
  (return (`|EnumEquality` (`self.CellState`) "NewEnumerator2")))

(fn `IsStillInFireRange`
  (returns (ReturnValue :type Boolean))
  (return (< (`self.FireDistance`) (`self.FireRange`))))

(fn `OnMerged`
  ;[1 1 1] Increase resource value
  (set `self.ResourceValue` (* (`self.ResourceValue`) 2))
  ;[1 1 1] Update flipbook
  (`self.UpdateResourceFlipbook`)
  ;[1 1 1] Play merge sound
  (`self.PlayRandom` (`|MakeArray` (`self.merge1`) (`self.merge2`) (`self.merge3`) (`self.merge4`))))

(fn `PlayRandom`
  (params (`[0]` :type "Array of AudioComponent Object Reference"))
  (`AudioComponent.Play` (`|GetArrayItem` `[0]` (`KismetMathLibrary.RandomInteger` (`KismetArrayLibrary.Array_Length` `[0]`))) 0.0))

(fn `SetFree`
  (set `self.CellState` "NewEnumerator0")
  (set `self.CurrentPlayer` null)
  (`PrimitiveComponent.SetCollisionResponseToChannel` (`self.Box`) "ECC_Pawn" "ECR_Overlap")
  (`PaperFlipbookComponent.SetFlipbook` (`self.Flipbook`) "/Game/Graphics/Space/Flipbooks/FP_empty.FP_empty"))

(fn `SetHighlighted`
  (params (IsHighlighted :type Boolean))
  (if IsHighlighted
    (`PaperFlipbookComponent.SetFlipbook` (`self.Flipbook`) "/Game/Graphics/Space/Flipbooks/FP_selected.FP_selected")
    (else
      (`self.SetSelected` (`|EnumEquality` (`self.CellState`) "NewEnumerator2")))))

(fn `SetSelected`
  (params (IsReady :type Boolean))
  (if IsReady
    (set `self.CellState` "NewEnumerator2")
    (`PaperFlipbookComponent.SetFlipbook` (`self.Flipbook`) "/Game/Graphics/Space/Flipbooks/FP_selected.FP_selected")
    (else
      (set `self.CellState` "NewEnumerator1")
      (`PaperFlipbookComponent.SetFlipbook` (`self.Flipbook`) "/Game/Graphics/Space/Flipbooks/FP_attracted.FP_attracted"))))

(fn `SetSlag`
  (set `self.CurrentPlayer` null)
  (set `self.FireDistance` 0.0)
  (set `self.FireDirection` (0.0 0.0 0.0))
  (set `self.FireForce` 0.0)
  (`self.K2_SetActorLocation` (`KismetMathLibrary.Conv_IntVectorToVector` (`KismetMathLibrary.FTruncVector` (`self.K2_GetActorLocation`))) false true)
  (`PrimitiveComponent.SetCollisionResponseToChannel` (`self.Box`) "ECC_Pawn" "ECR_Overlap")
  (set `self.CellState` "NewEnumerator4")
  (`KismetSystemLibrary.K2_SetTimer` null "SetFree" (`self.SlagToFreeTime`)))

(fn `UpdateResourceFlipbook`
  (locals (UnknownResource :type "PaperFlipbook Object Reference" :default "PaperFlipbook'/Game/Graphics/Space/Flipbooks/FP_resource_error.FP_resource_error'"))
  (bind _value (`BlueprintMapLibrary.Map_Find` (`|MakeMap` 1 "/Game/Graphics/Space/Flipbooks/FP_ore1.FP_ore1" 2 "/Game/Graphics/Space/Flipbooks/FP_ore2.FP_ore2" 4 "/Game/Graphics/Space/Flipbooks/FP_ore4.FP_ore4" 8 "/Game/Graphics/Space/Flipbooks/FP_ore8.FP_ore8" 16 "/Game/Graphics/Space/Flipbooks/FP_ore16.FP_ore16" 32 "/Game/Graphics/Space/Flipbooks/FP_metal1.FP_metal1" 64 "/Game/Graphics/Space/Flipbooks/FP_metal2.FP_metal2" 128 "/Game/Graphics/Space/Flipbooks/FP_metal4.FP_metal4" :!valuetype "PaperFlipbook Object Reference") (`self.ResourceValue`)))
  (`/Engine/EditorBlueprintResources/StandardMacros.IsValid` _value
    (:`Is Valid`
      (`PaperFlipbookComponent.SetFlipbook` (`self.Resource`) _value))
    (:`Is Not Valid`
      (`PaperFlipbookComponent.SetFlipbook` (`self.Resource`) (`local.UnknownResource`)))))

(fn `UserConstructionScript`)