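; BP_InputsManager handles input for offensive mode and for switching between two players.
; Pressing and releasing the OffensiveMode action fires enabled and disabled event dispatchers.
; SwitchPlayer toggles the index between 0 and 1, looks it up in Players and blends player controller 0's view to that target, printing a message if none is found.
; Only the camera changes, as the possess and unpossess nodes never run.
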(event `InputAction|OffensiveMode`
  (params (Key :type "Key Structure"))
  ;[1 1 1] Offensive mode
  (:`Pressed`
    (`self.OnOffensiveModeEnabled`))
  (:`Released`
    (`self.OnOffensiveModeDisabled`)))

(event `InputAction|SwitchPlayer`
  (params (Key :type "Key Structure"))
  (bind (_value _returnvalue) (`BlueprintMapLibrary.Map_Find` (`self.Players`) (`self.CurrentPlayerIndex`)))
  ;[1 1 1] Player switch
  (:`Pressed`
    (set `self.CurrentPlayerIndex` (mod (+ (`self.CurrentPlayerIndex`) 1) 2))
    (if _returnvalue
      (`PlayerController.SetViewTargetWithBlend` (`GameplayStatics.GetPlayerController` 0) _value 0.5 "VTBlend_Linear" 0.0 false)
      (else
        (`self.PrintValue` (`KismetStringLibrary.Conv_IntToString` (`self.CurrentPlayerIndex`)) "No player found at current index. Please fill players array. Index:")))))

(fn `PrintValue`
  (params (Value :type String) (Meesage :type String))
  (`KismetSystemLibrary.PrintString` (`KismetStringLibrary.Concat_StrStr` Meesage Value)))

(fn `UserConstructionScript`)