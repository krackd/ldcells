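; BP_EnergyCell is an energy cell pickup that can attach to a player and becomes a shield cell while attached.
; AttachToPlayer and DettachFromPlayer store or clear the owning player and swap the Paper2D flipbook between energy and shield looks.
; While attached, its box overlap makes the player attract any unattached cell it touches, chaining pickups, and cancels the player's move when it hits a BP_Wall.
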(event `self.Box.OnComponentBeginOverlap`
  (params (OverlappedComponent :type "PrimitiveComponent Object Reference") (OtherActor :type "Actor Object Reference") (OtherComp :type "PrimitiveComponent Object Reference") (OtherBodyIndex :type Integer) (bFromSweep :type Boolean) (SweepResult :type "HitResult Structure (by ref)"))
  (`|ExecutionSequence`
    (:`then_0`
      (bind _asbp_energy_cell (cast `/Game/Blueprints/BP_EnergyCell` OtherActor))
      (if (and (`self.IsAttachedToPlayer`) (not (`/Game/Blueprints/BP_EnergyCell.IsAttachedToPlayer` _asbp_energy_cell)))
        (`/Game/Blueprints/BP_Custom_Player.AttractEnergyCell` (`self.CurrentPlayer`) _asbp_energy_cell)))
    (:`then_1`
      (cast `/Game/Blueprints/BP_Wall` OtherActor)
      (if (`self.IsAttachedToPlayer`)
        (`/Game/Blueprints/BP_Custom_Player.CancelMove` (`self.CurrentPlayer`))))))

(fn `AttachToPlayer`
  (params (Player :type "/Game/Blueprints/BP_Custom_Player Object Reference"))
  (set `self.CurrentPlayer` Player)
  (set `self.IsAttachedToPlayer` true)
  (`PaperFlipbookComponent.SetFlipbook` (`self.Flipbook`) "/Game/Graphics/Cells/Small/Flipbooks/FP_SheildCell.FP_SheildCell"))

(fn `DettachFromPlayer`
  (set `self.CurrentPlayer` null)
  (set `self.IsAttachedToPlayer` false)
  (`PaperFlipbookComponent.SetFlipbook` (`self.Flipbook`) "/Game/Graphics/Cells/Small/Flipbooks/FP_EnergyCell.FP_EnergyCell"))

(fn `UserConstructionScript`)